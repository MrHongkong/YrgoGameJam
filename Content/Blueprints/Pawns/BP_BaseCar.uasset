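; Base car pawn that drives by pushing a physics ball with force along a yaw direction set by steering input.
; Each tick the attached components follow the ball, the car root faces the steering direction, and the spring arm eases its yaw toward it.
; Lap and checkpoint values are stored through interface calls.
; Slide effects and slope alignment are unwired; the active ground trace only prints distance.
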(event EventTick
  (params (DeltaSeconds :type Float%20%28single-precision%29))
  (bind _ball (Variables|Default|GetBall))
  ;[1 1 1] Update things
  (Transformation|SetWorldLocation (Variables|Default|GetAttachedToBall) (Transformation|GetWorldLocation _ball) false false)
  (bind _output_get (Variables|Default|SetBallDirection (Math|Conversions|RotationFromXVector (Transformation|GetComponentVelocity _ball))))
  (Transformation|SetWorldRotation (Variables|Default|GetArrow) _output_get false false)
  (Transformation|SetWorldRotation (Variables|Default|GetCarRoot) (Variables|Default|GetCarDirection) false false)
  (Variables|Default|SetVelocityDirection (Math|Vector|Normalize (Transformation|GetComponentVelocity _ball)))
  (CallFunction|LineTracetoGround)
  (CallFunction|LerpCameratoDirection))

(event EventISetCheckpoint
  (params (cpi :type Integer))
  ;[1 1 1] Lap/Checkpoint interface thingamabobs
  (Variables|Default|Setcheckpoints cpi))

(event EventBeginPlay
  ;[1 1 1] BeginPlay
  (Components|Activation|Deactivate (Variables|Default|GetSlide1)))

(event EventISetLap
  (params (lap :type Integer))
  ;[1 1 1] Lap/Checkpoint interface thingamabobs
  (Variables|Default|Setlaps lap))

(event Input|AxisEvents|InputAxisMoveForward
  (params (AxisValue :type Float%20%28single-precision%29))
  ;[1 1 1] Accelerate
  (Physics|AddForce (Variables|Default|GetBall) (* (Math|Vector|GetForwardVector (Variables|Default|GetCarDirection)) (* AxisValue (Variables|Default|GetaccelerationForce))) "None" false))

(event Input|AxisEvents|InputAxisMoveRight
  (params (AxisValue :type Float%20%28single-precision%29))
  ;[1 1 1] Turn
  (Variables|Default|SetCarDirection (Math|Rotator|MakeRotator 0.0 0.0 (+ (* AxisValue (Variables|Default|GetturnSpeed)) (.yaw (Variables|Default|GetCarDirection))))))

(fn ConstructionScript)

(fn SlideyFunction
  (bind _cardirection (Variables|Default|GetCarDirection))
  (bind _velocitydirection (Variables|Default|GetVelocityDirection))
  (bind _slide1 (Variables|Default|GetSlide1))
  (bind _returnvalue (Math|Vector|GetForwardVector _cardirection))
  (bind _returnvalue_2 (- _returnvalue _velocitydirection))
  (Math|Float|CompareFloat (+ (Math|Float|Absolute(Float) (.x _returnvalue_2)) (Math|Float|Absolute(Float) (.y _returnvalue_2))) 0.75
    (:>
      (bind _output_get (Variables|Default|SetnewValue true)))
    (:<
      (Variables|Default|SetnewValue false)))
  (if (not _output_get)
    (if _output_get
      (Components|Activation|Activate _slide1 false)
      (Variables|Default|SetisSliding true)
      (else
        (Components|Activation|Deactivate _slide1)
        (Variables|Default|SetisSliding false)))))

(fn AdjusttoSurfaceNormal
  (bind _ball (Variables|Default|GetBall))
  (bind _returnvalue (Transformation|GetWorldLocation _ball))
  (bind (_outhit _returnvalue_2) (Collision|LineTraceForObjects _returnvalue (+ _returnvalue "0, 0,-1000.000000") (Utilities|Array|MakeArray "ObjectTypeQuery1" "ObjectTypeQuery2" "ObjectTypeQuery3" "ObjectTypeQuery4" "ObjectTypeQuery5") false 0 "None"))
  (if _returnvalue_2
    (Transformation|SetRelativeRotation (Variables|Default|GetCarMesh) (Math|Rotator|MakeRotator (.OutSlopePitchDegreeAngle (Class|KismetMathLibrary|GetSlopeDegreeAngles (Math|Vector|GetRightVector (Variables|Default|GetCarRoot)) (.Normal (Collision|BreakHitResult _outhit)) (Math|Vector|MakeVector 0.0 0.0 1.0))) (* (.OutSlopePitchDegreeAngle (Class|KismetMathLibrary|GetSlopeDegreeAngles (Math|Vector|GetRightVector (Variables|Default|GetCarRoot)) (.Normal (Collision|BreakHitResult _outhit)) (Math|Vector|MakeVector 0.0 0.0 1.0))) -1.0) 0.0) false false)))

(fn LineTracetoGround
  (bind _ball (Variables|Default|GetBall))
  (bind _returnvalue (Transformation|GetWorldLocation _ball))
  (bind _outhit (Collision|LineTraceForObjects _returnvalue (+ _returnvalue "0, 0,-1000.000000") (Utilities|Array|MakeArray "ObjectTypeQuery1" "ObjectTypeQuery2" "ObjectTypeQuery3" "ObjectTypeQuery4" "ObjectTypeQuery5") false 0 "None"))
  (Development|PrintString (Utilities|String|ToString(Float) (.distance _outhit))))

(fn LerpCameratoDirection
  (bind _springarm (Variables|Default|GetSpringArm))
  (Transformation|SetRelativeRotation _springarm (Math|Rotator|MakeRotator 0.0 (.pitch (Variables|/Script/Engine.SceneComponent|GetRelativeRotation _springarm)) (.yaw (Math|Conversions|RotationFromXVector (Math|Vector|GetForwardVector (Class|KismetMathLibrary|RInterptoConstant (Transformation|GetWorldRotation _springarm) (Variables|Default|GetCarDirection) (Utilities|Time|GetWorldDeltaSeconds) (Variables|Default|GetcameraFollowSpeed)))))) false false))

(fn IGetCheckpoint
  (return (Variables|Default|Getcheckpoints)))

(fn IGetLap
  (return (Variables|Default|Getlaps)))