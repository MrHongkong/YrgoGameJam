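; Checkpoint actor for a lap race that tracks each overlapping actor's progress and detects the winner.
; On overlap, with a valid checkpoint system reference, it accepts only the next checkpoint index in sequence, wrapping from last to first.
; It stores progress on the actor through interface messages.
; A checkpoint flagged as finish also increments the lap and fires the game system's win event when the count equals the required laps.
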(event Collision|EventActorBeginOverlap
  (params (OtherActor :type Actor%20Object%20Reference))
  ;[1 1 1] Sysref Valid Check
  (bind _valid (CallFunction|CheckCpsys))
  (if _valid
    ;[1 1 1] Check Checkpoint
    (bind _result (CallFunction|CheckCheckpoint OtherActor))
    (if _result
      ;[1 1 1] Update Checkpoint for Player
      (CallFunction|UpdateCheckpoint OtherActor)
      ;[1 1 1] Check Finish
      (bind _finish (CallFunction|CheckFinish))
      (if _finish
        ;[1 1 1] Update Lap for Player
        (bind _laps (CallFunction|UpdateLap OtherActor))
        ;[1 1 1] Check Win for Player
        (bind _win (CallFunction|CheckWin _laps))
        (if _win
          ;[1 1 1] Win Event
          (Default|WinEvent (Variables|/Game/Filip/BP_CP_System.BP_CP_System_C|Getgsys (Variables|Default|Getcpsys)) OtherActor))))))

(fn ConstructionScript)

(fn UpdateCheckpoint
  (params (otherActor :type Actor%20Object%20Reference))
  (Class|ICheckpointable|ISetCheckpoint(Message) otherActor (Variables|Default|Getcpi)))

(fn CheckCpsys
  ;[1 1 1] Sysref Valid Check
  (if (Utilities|IsValid (Variables|Default|Getcpsys))
    (return true)
    (else
      (return false))))

(fn CheckWin
  (params (laps :type Integer))
  (if (== laps (Variables|/Game/Filip/BP_Game_System.BP_Game_System_C|GetrequiredLaps (Variables|/Game/Filip/BP_CP_System.BP_CP_System_C|Getgsys (Variables|Default|Getcpsys))))
    (return true)
    (else
      (return false))))

(fn UpdateLap
  (params (otherActor :type Actor%20Object%20Reference))
  (LocalVariables|SetlocalOtherActor otherActor)
  (bind _lap (Class|ILappable|IGetLap(Message) (LocalVariables|GetlocalOtherActor)))
  (Class|ILappable|ISetLap(Message) (LocalVariables|GetlocalOtherActor) (+ _lap 1))
  (return (+ _lap 1)))

(fn CheckCheckpoint
  (params (otherActor :type Actor%20Object%20Reference))
  (bind _cpi (Class|ICheckpointable|IGetCheckpoint(Message) otherActor))
  (if (or (== _cpi (- (Variables|Default|Getcpi) 1)) (and (== _cpi (- (Utilities|Array|Length (Variables|/Game/Filip/BP_CP_System.BP_CP_System_C|Getcps (Variables|Default|Getcpsys))) 1)) (== (Variables|Default|Getcpi) 0)))
    (return true)
    (else
      (return false))))

(fn CheckFinish
  (if (Variables|Default|Getfinish)
    (return true)
    (else
      (return false))))