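; BP_CP_System is a manager for BP_CP actors, apparently race checkpoints, that registers them and marks the finish.
; Its Setup function clears the Cps array, gathers every BP_CP in the level into it and gives each a back-reference to the system.
; A second pass sets Finish to true on any checkpoint whose Cpi index is zero and false on the rest.
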(fn ConstructionScript)

(fn Setup
  (Utilities|Array|Clear (Variables|Default|Getcps))
  (bind _outactors (Actor|GetAllActorsOfClass "/Game/Filip/BP_CP.BP_CP_C"))
  (for _array_element _outactors
    (Variables|/Game/Filip/BP_CP.BP_CP_C|Setcpsys _array_element self)
    (Utilities|Array|Add (Variables|Default|Getcps) _array_element))
  (for (_array_element_2 _array_index) (Variables|Default|Getcps)
    (if (== (Variables|/Game/Filip/BP_CP.BP_CP_C|Getcpi (Utilities|Array|Get(acopy) (Variables|Default|Getcps) _array_index)) 0)
      (Variables|/Game/Filip/BP_CP.BP_CP_C|Setfinish _array_element_2 true)
      (else
        (Variables|/Game/Filip/BP_CP.BP_CP_C|Setfinish _array_element_2 false)))))