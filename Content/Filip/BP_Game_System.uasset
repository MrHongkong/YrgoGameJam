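; Game manager actor that handles checkpoint setup, player respawns and the win screen for what appears to be a ball-and-car race.
; On BeginPlay it uses its assigned or first-found BP_CP_System and runs its setup.
; RespawnPlayer matches the player's checkpoint, teleports the ball above it, toggles physics and aligns both directions to the checkpoint's right vector.
; WinEvent shows the winning controller a win widget with mouse input.
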(event Custom|WinEvent
  (params (winningActor :type Actor%20Object%20Reference))
  (Development|PrintString (Utilities|String|Append (Utilities|GetDisplayName winningActor) " you win!"))
  (bind _asplayer_controller (Utilities|Casting|CastToPlayerController winningActor))
  (Input|SetInputModeGameandUI _asplayer_controller 0 "DoNotLock" true)
  (Variables|/Script/Engine.PlayerController|SetbShowMouseCursor _asplayer_controller true)
  (bind _returnvalue (UserInterface|CreateWidget "/Game/MenuContents/BP_WinScreenWidget.BP_WinScreenWidget_C" _asplayer_controller))
  (UserInterface|Viewport|AddtoViewport _returnvalue 0)
  (Default|SetWinnner _returnvalue _asplayer_controller))

(event Custom|RespawnPlayer
  (params (player :type BP%20Base%20Car%20Object%20Reference))
  (bind _ball (Variables|/Game/Blueprints/Pawns/BP_BaseCar.BP_BaseCar_C|GetBall player))
  (bind _cpi (Class|ICheckpointable|IGetCheckpoint(Message) player))
  (bind _array_element (Utilities|Array|ForEachLoopwithBreak (Variables|/Game/Filip/BP_CP_System.BP_CP_System_C|Getcps (Variables|Default|Getcpsys)) :!label _label)
    (:LoopBody
      (if (== _cpi (Variables|/Game/Filip/BP_CP.BP_CP_C|Getcpi _array_element))
        (Transformation|SetWorldTransform _ball (Math|Transform|MakeTransform (+ (Math|Vector|MakeVector 0.0 0.0 (* 100 (.Z (Math|Vector|BreakVector (.Scale (Math|Transform|BreakTransform (Transformation|GetActorTransform _array_element))))))) (.Location (Math|Transform|BreakTransform (Transformation|GetActorTransform _array_element)))) (.Rotation (Math|Transform|BreakTransform (Transformation|GetActorTransform _array_element))) (Variables|/Script/Engine.SceneComponent|GetRelativeScale3D _ball)) false true)
        (Physics|SetSimulatePhysics _ball false)
        (Physics|SetSimulatePhysics _ball true)
        (Variables|/Game/Blueprints/Pawns/BP_BaseCar.BP_BaseCar_C|SetBallDirection player (Math|Conversions|RotationFromXVector (Math|Vector|GetRightVector (.Rotation (Math|Transform|BreakTransform (Transformation|GetActorTransform _array_element))))))
        (Variables|/Game/Blueprints/Pawns/BP_BaseCar.BP_BaseCar_C|SetCarDirection player (Math|Conversions|RotationFromXVector (Math|Vector|GetRightVector (.Rotation (Math|Transform|BreakTransform (Transformation|GetActorTransform _array_element))))))
        (goto _label Break)))))

(event EventBeginPlay
  (CallFunction|SetupCpsys))

(fn ConstructionScript)

(fn SetupCpsys
  (if (Utilities|IsValid (Variables|Default|Getcpsys))
    (Variables|/Game/Filip/BP_CP_System.BP_CP_System_C|Setgsys (Variables|Default|Getcpsys) self :!label _label)
    (Default|Setup (Variables|Default|Getcpsys) :!label _label_2)
    (else
      (bind _outactors (Actor|GetAllActorsOfClass "/Game/Filip/BP_CP_System.BP_CP_System_C"))
      (if (> (Utilities|Array|Length _outactors) 0)
        (Variables|Default|Setcpsys (Utilities|Array|Get(acopy) _outactors))
        (if (Utilities|IsValid (Variables|Default|Getcpsys))
          (goto _label)
          (else
            (bind _returnvalue (Game|SpawnActorfromClass "/Game/Filip/BP_CP_System.BP_CP_System_C" (Transformation|GetWorldTransform (Variables|Default|GetDefaultSceneRoot)) "Undefined" 0 0 self 0))
            (Variables|Default|Setcpsys _returnvalue)
            (goto _label_2)))))))